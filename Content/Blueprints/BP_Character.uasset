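; Player character with camera-relative movement, look and jump, which also controls which doors in the level are open.
; Axis inputs move along the camera's forward and right vectors and feed controller pitch and yaw.
; On BeginPlay it calls a function to randomise all door indices.
; The hard-bound A key cycles the open index through four values and passes it to SetOpenDoorIndex.
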(event `self.ReceiveBeginPlay`
  (`MyBlueprintFunctionLibrary.RandomiseAllDoorsIndexs`))

(event `InputAxis|MoveForward`
  (params (AxisValue :type "Float (single-precision)"))
  (`self.AddMovementInput` (`SceneComponent.GetForwardVector` (`self.Camera`)) AxisValue))

(event `InputAxis|MoveRight`
  (params (AxisValue :type "Float (single-precision)"))
  (`self.AddMovementInput` (`SceneComponent.GetRightVector` (`self.Camera`)) AxisValue))

(event `InputAxis|LookUp`
  (params (AxisValue :type "Float (single-precision)"))
  (`self.AddControllerPitchInput` AxisValue))

(event `InputAxis|LookRight`
  (params (AxisValue :type "Float (single-precision)"))
  (`self.AddControllerYawInput` AxisValue))

(event `InputAction|Jump`
  (params (Key :type "Key Structure"))
  (:`Pressed`
    (`self.Jump`)))

(event `Key|A`
  (params (Key :type "Key Structure"))
  (:`Pressed`
    (bind _output_get (set `self.CurrentOpenedIndex` (mod (+ (`self.CurrentOpenedIndex`) 1) 4)))
    (`MyBlueprintFunctionLibrary.SetOpenDoorIndex` _output_get)))

(fn `UserConstructionScript`)